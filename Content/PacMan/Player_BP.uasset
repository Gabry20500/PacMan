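; Player pawn Blueprint for a Pac-Man game that keeps moving in the last direction the player chose.
; Forward and lateral axis inputs only set a Direction value when non-zero, so releasing the input does not stop movement.
; Each Tick switches on Direction and adds full movement input along the matching positive or negative world X or Y axis.
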(event `self.ReceiveTick`
  (params (DeltaSeconds :type "Float (single-precision)"))
  (switch `int` (`self.Direction`)
    (:`1`
      (bind _output_get (set `self.force` 1.0))
      (`self.AddMovementInput` (`KismetMathLibrary.MakeVector` _output_get)))
    (:`2`
      (bind _output_get_2 (set `self.force` -1.0))
      (`self.AddMovementInput` (`KismetMathLibrary.MakeVector` _output_get_2)))
    (:`3`
      (bind _output_get_3 (set `self.force` 1.0))
      (`self.AddMovementInput` (`KismetMathLibrary.MakeVector` 0.0 _output_get_3)))
    (:`4`
      (bind _output_get_4 (set `self.force` -1.0))
      (`self.AddMovementInput` (`KismetMathLibrary.MakeVector` 0.0 _output_get_4)))))

(event `InputAxis|MoveForeward`
  (params (AxisValue :type "Float (single-precision)"))
  ;[1 1 1] Move Forward
  (if (== AxisValue 0.0)
    _
    (elif (not (<= AxisValue 0.0))
      (set `self.Direction` 1)
      (else
        (set `self.Direction` 2)))))

(event `InputAxis|MoveLateral`
  (params (AxisValue :type "Float (single-precision)"))
  ;[1 1 1] Move Lateral
  (if (== AxisValue 0.0)
    _
    (elif (not (<= AxisValue 0.0))
      (set `self.Direction` 3)
      (else
        (set `self.Direction` 4)))))

(fn `UserConstructionScript`)